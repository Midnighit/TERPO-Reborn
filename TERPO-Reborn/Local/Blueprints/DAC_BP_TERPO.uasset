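; DAC_BP_TERPO is a command handler for the TERPO mod that reports a Funcom ID.
; DoCommand stores the parameters and calling controller, casts it to FunCombat_PlayerController, and fetches its FCPC_AC_TERPO component.
; It switches on the first parameter and calls GetFuncomId, which prints the component's Funcom ID with on-screen display disabled.
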(event `self.DoCommand`
  (params (Parameters :type "Array of String (by ref)") (CallingPlayerController :type "ConanPlayerController Object Reference") (World :type "World Object Reference"))
  (set `self.parameters` Parameters)
  (bind _output_get (set `self.PC_Ref` CallingPlayerController))
  (bind _asfun_combat_player_controller (cast `/Game/Systems/FunCombat_PlayerController` _output_get))
  (set `self.FCPC_AC_Ref` (`self.GetComponentByClass` _asfun_combat_player_controller "/Game/Mods/TERPO-Reborn/ActorComponents/FCPC_AC_TERPO.FCPC_AC_TERPO_C"))
  (switch `string` (`KismetArrayLibrary.Array_Get` (`self.parameters`))
    (:`getFuncomId`
      (`KismetSystemLibrary.PrintText` (`KismetTextLibrary.Conv_StringToText` (`/Game/Mods/TERPO-Reborn/ActorComponents/FCPC_AC_TERPO.GetFuncomId` (`self.FCPC_AC_Ref`))) false))))

(fn `UserConstructionScript`)