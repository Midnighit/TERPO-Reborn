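; TERPO placeable building Blueprint for Conan that adds a shareable state on top of the ownership check.
; CheckForOwner passes owners or anyone when shared or always shared, suppressing the GUI notification for containers, ignorable ownership and shared objects.
; SetIsShared, skipped when always shared, relays the change through the local player character's BPC_AC_BP_TERPO component RPC.
; ServerSetIsShared stores the flag and marks building persistence dirty with a delay.
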(event `Server SetIsShared`
  (params (IsShared :type Boolean))
  ;[1 0 0] Server Set IsShared
  (set `self.isShared` IsShared)
  (`PersistenceComponent.SetDirty` (`self.ConanBuildingPersistence`) true 5.0))

(fn `CheckForOwner`
  (params (Instigator :type "PlayerController Object Reference") (HitIndex :type Integer))
  (returns (Instigator_Out :type "PlayerController Object Reference") (HitIndex_Out :type Integer) (IsOwner :type Boolean))
  (bind _isshared (`self.isShared`))
  (bind _isalwaysshared (`self.isAlwaysShared`))
  (return Instigator HitIndex (or (`self.IsOwner` (`Controller.K2_GetPawn` Instigator) (not (or (`self.GetIsContainer`) (`self.CanIgnoreOwnership`) _isshared _isalwaysshared))) _isshared _isalwaysshared)))

(fn `SetIsShared`
  (params (IsShared :type Boolean))
  (if (not (`self.isAlwaysShared`))
    (`/Game/Mods/TERPO-Reborn/ActorComponents/BPC_AC_BP_TERPO.RPC SetIsShared` (`KismetArrayLibrary.Array_Get` (`self.K2_GetComponentsByClass` (`GameplayStatics.GetPlayerCharacter` 0) "/Game/Mods/TERPO-Reborn/ActorComponents/BPC_AC_BP_TERPO.BPC_AC_BP_TERPO_C")) self IsShared)
    (return)
    (else
      (return))))

(fn `UserConstructionScript`
  (`parent.UserConstructionScript`))