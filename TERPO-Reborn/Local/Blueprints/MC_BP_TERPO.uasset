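; TERPO mod controller (apparently for character slots) that merges the mod's UI modules and activates its menu alongside the in-game menu.
; On BeginPlay it waits for match start (server) or a valid character (client) before signalling readiness.
; It tracks each player's named slots and active slot, and exposes slot-limit, admin-slot and beehive-lock settings.
; Database writes are queued and drained once per second by a looping timer that dirties the persistence component.
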(event `WaitTillMatchIsStarted`
  ;[1 0 0] Wait for Server to get ready
  (if (`GameStateBase.HasMatchStarted` (`GameplayStatics.GetGameState`))
    (`KismetSystemLibrary.K2_ClearAndInvalidateTimerHandle` (`self.WaitForMatchStartedLoop`))
    (`self.SetActorTickEnabled` false :!label _label)
    ;[1 1 1] End of normal loading chain
    (set `self.ModControllerFullyExecuted` true)
    (`self.OnModControllerFullyExecuted`)
    ;[1 1 1] Make the TERPO menu show when the Ingame Menu is opened
    (if (not (`KismetSystemLibrary.IsDedicatedServer`))
      (bind _returnvalue (`GUIModuleController.GetModule` (`GUIModuleController.GetGUIModuleController`) "IngameMenu"))
      (add `GUIModule.SignalActivated` _returnvalue (delegate `IngameMenuOpened`)))))

(event `self.ReceiveBeginPlay`
  (if (`KismetSystemLibrary.IsServer`)
    ;[1 0 0] Wait for Server to get ready
    (bind _returnvalue (`KismetSystemLibrary.K2_SetTimerDelegate` (delegate `WaitTillMatchIsStarted`) 0.5 true))
    (set `self.WaitForMatchStartedLoop` _returnvalue)
    (else
      ;[0 1 0] Wait for Client to get ready
      (bind _returnvalue_2 (`KismetSystemLibrary.K2_SetTimerDelegate` (delegate `WaitForValidPlayerController`) 1.0 true))
      (set `self.WaitForPlayerControllerTime` _returnvalue_2))))

(event `WaitForValidPlayerController`
  ;[0 1 0] Wait for Client to get ready
  (`/Engine/EditorBlueprintResources/StandardMacros.IsValid` (`GameplayStatics.GetPlayerCharacter` 0)
    (:`Is Valid`
      (`KismetSystemLibrary.K2_ClearAndInvalidateTimerHandle` (`self.WaitForPlayerControllerTime`))
      (goto _label))))

(event `IngameMenuOpened`
  (params (module :type "GUIModule Object Reference") (isActive :type Boolean))
  ;[1 1 1] Make the TERPO menu show when the Ingame Menu is opened
  (bind _returnvalue (`GUIModuleController.ActivateModule` (`GUIModuleController.GetGUIModuleController`) "Menu_TERPO" isActive false))
  (cast `/Game/Mods/TERPO-Reborn/Widgets/CharSelect_W_TERPO` _returnvalue))

(event `DatabaseQueueElementAdded`
  ;[1 0 0] Write queue to DB until empty
  (`self.SetActorTickEnabled` true)
  (bind _returnvalue (`KismetSystemLibrary.K2_SetTimer` null "ProcessDatabaseQueue" 1.0 true))
  (set `self.throttleDatabaseAccss` _returnvalue))

(fn `AddToDatabaseQueue`
  (params (queueElement :type "/Game/Mods/TERPO-Reborn/Variables/PassToDB_STRUCT_TERPO Structure"))
  (`KismetArrayLibrary.Array_Add` (`self.DatabaseQueue`) queueElement)
  (`self.DatabaseQueueElementAdded`)
  (return))

(fn `GetActiveSlot`
  (params (playerId :type String))
  (returns (index :type Integer) (slot :type Integer))
  (locals (arrayIndex :type Integer) (playerIdFound :type Boolean))
  (bind _arrayindex (`local.arrayIndex`))
  (set `local.playerIdFound` false) ; Initialize playerIdFound\nto false
  (set `local.arrayIndex` -1) ; Initialze array\nindex to -1
  (for (_array_element _array_index) (`self.charSlots`)
    (bind (_playerid _slotnum _slotname _isactive) (break `/Game/Mods/TERPO-Reborn/Variables/CharSlots_STRUCT_TERPO` _array_element))
    (if (`KismetStringLibrary.EqualEqual_StrStr` playerId _playerid)
      (if _isactive
        (set `local.arrayIndex` _array_index) ; Remember array\nindex of active slot
        (break)
        (else
          (set `local.playerIdFound` true) ; Remember if playerId was\nfound but not active slot
        ))))
  (if (>= _arrayindex 0)
    (return _arrayindex _slotnum) ; Array index was found
    (elif (not (`local.playerIdFound`))
      (bind _returnvalue (`KismetArrayLibrary.Array_Add` (`self.charSlots`) (make `/Game/Mods/TERPO-Reborn/Variables/CharSlots_STRUCT_TERPO` playerId 1 "" true))) ; Array index wasn't found.\n-> add new array element
      (return _returnvalue 1)
      (else
        (`LoggerLibrary.DWLogString` "TERPO (MC_BP in GetActiveSlot): playerId but no active slot found!" "Modding" "INFOL_INFO0" true) ; playerId found, active slot not found.\nShould never get here!!!
        (return -1 -1)))))

(fn `GetAdminSlotEnabled`
  (returns (AdminSlotEnabled :type Boolean))
  (return (`self.AdminSlotEnabled`)))

(fn `GetBeehiveImprIsLockable`
  (returns (BeehiveImprIsLockable :type Boolean))
  (return (`self.BeehiveImprIsLockable`)))

(fn `GetBeehiveIsLockable`
  (returns (IsLockable :type Boolean))
  (return (`self.BeehiveIsLockable`)))

(fn `GetMaxSlot`
  (returns (maxSlots :type Integer))
  (return (`self.maxSlots`)))

(fn `GetSlotName`
  (params (playerId :type String) (slotNum :type Integer))
  (returns (index :type Integer) (slotName :type String))
  (locals (arrayIndex :type Integer))
  (bind _arrayindex (`local.ArrayIndex`))
  (set `local.arrayIndex` -1)
  (for (_array_element _array_index) (`self.charSlots`)
    (bind (_playerid _slotnum _slotname) (break `/Game/Mods/TERPO-Reborn/Variables/CharSlots_STRUCT_TERPO` _array_element))
    (`/Game/Systems/BP_MacroGlobal.And+Branch` (== slotNum _slotnum) (`KismetStringLibrary.EqualEqual_StrStr` playerId _playerid)
      (:`True`
        (set `local.arrayIndex` _array_index)
        (break))))
  (if (>= (`local.ArrayIndex`) 0)
    (return _arrayindex _slotname) ; Array index was found
    (else
      (return _arrayindex "") ; Array index wasn't found
    )))

(fn `ModDataTableOperations`
  (`self.MergeDataTables` "/Game/UI/UIModuleTable.UIModuleTable" "/Game/Mods/TERPO-Reborn/Tables/UIModule_DT_TERPO.UIModule_DT_TERPO"))

(fn `ProcessDatabaseQueue`
  (bind _databasequeue (`self.DatabaseQueue`))
  (set `self.passToDB` (`KismetArrayLibrary.Array_Get` (`self.DatabaseQueue`)))
  (`PersistenceComponent.SetDirty` (`self.PersistenceComponent`) true 0.1)
  (`KismetArrayLibrary.Array_Remove` _databasequeue)
  (if (== (`KismetArrayLibrary.Array_Length` _databasequeue) 0)
    (`KismetSystemLibrary.K2_ClearAndInvalidateTimerHandle` (`self.throttleDatabaseAccss`))
    (`self.SetActorTickEnabled` false)))

(fn `SetActiveSlot`
  (params (playerId :type String) (slotNum :type Integer))
  (returns (index :type Integer))
  (locals (ArrayIndex :type Integer))
  (bind _charslots (`self.charSlots`))
  (set `local.ArrayIndex` -1) ; Initialze array\nindex to -1
  (for (_array_element _array_index) (`self.charSlots`)
    (bind (_playerid _slotnum _slotname) (break `/Game/Mods/TERPO-Reborn/Variables/CharSlots_STRUCT_TERPO` _array_element))
    (if (`KismetStringLibrary.EqualEqual_StrStr` playerId _playerid)
      (if (== slotNum _slotnum)
        (`KismetArrayLibrary.Array_Set` _charslots _array_index (make `/Game/Mods/TERPO-Reborn/Variables/CharSlots_STRUCT_TERPO` _playerid _slotnum _slotname true)) ; Correct slot, set to active
        (set `local.ArrayIndex` _array_index) ; Remember array index
        (else
          (`KismetArrayLibrary.Array_Set` _charslots _array_index (make `/Game/Mods/TERPO-Reborn/Variables/CharSlots_STRUCT_TERPO` _playerid _slotnum _slotname false)) ; Wrong slot, set to inactive
        ))))
  (if (>= (`local.ArrayIndex`) 0)
    (return (`local.ArrayIndex`)) ; Array index was found
    (else
      (bind _returnvalue (`KismetArrayLibrary.Array_Add` (`self.charSlots`) (make `/Game/Mods/TERPO-Reborn/Variables/CharSlots_STRUCT_TERPO` playerId slotNum "" true))) ; Array index wasn't found\n-> add new array element
      (return _returnvalue))))

(fn `UserConstructionScript`)