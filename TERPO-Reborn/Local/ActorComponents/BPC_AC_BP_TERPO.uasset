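; Player character component for the TERPO mod in Conan Exiles that links the character to the mod controller and keeps the HUD visible in vanity camera.
; Outside dedicated servers, BeginPlay waits for the MC_BP_TERPO controller's fully-executed event, then runs client and server setup to cache references.
; Tick reapplies the HUD flag, retrying after a delay if the owner cast fails.
; SaveToDB stores player slot changes and marks character persistence dirty.
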(event `Retry Cast to BPC VC`
  ;[1 1 1] Prevent HUD from hiding when activating the vanity cam
  (bind _asbase_player_char (cast `/Game/Characters/BasePlayerChar` (`self.GetOwner`) :!label _label)
    (:`then`
      (set `/Game/Characters/BasePlayerChar.KeepHUDWhenInVanityCamera` true _asbase_player_char))
    (:`CastFailed`
      (`KismetSystemLibrary.Delay` 1.0)
      (`self.Retry Cast to BPC VC`))))

(event `self.ReceiveTick`
  (params (DeltaSeconds :type "Float (single-precision)"))
  ;[1 1 1] Prevent HUD from hiding when activating the vanity cam
  (goto _label))

(event `self.ReceiveBeginPlay`
  ;[0 1 0] Create ModControllerFullyExecuted Event
  (if (not (`KismetSystemLibrary.IsDedicatedServer`))
    (bind _outactors (`GameplayStatics.GetAllActorsOfClass` "/Game/Mods/TERPO-Reborn/MC_BP_TERPO.MC_BP_TERPO_C"))
    (bind _item (`KismetArrayLibrary.Array_Get` _outactors))
    (`/Engine/EditorBlueprintResources/StandardMacros.IsValid` _item
      (:`Is Valid`
        (set `self.ModController` _item)
        (add `/Game/Mods/TERPO-Reborn/MC_BP_TERPO.OnModControllerFullyExecuted` _item (delegate `On ModControllerFullyExecuted`))
        (if false
          (remove `/Game/Mods/TERPO-Reborn/MC_BP_TERPO.OnModControllerFullyExecuted` _item (delegate `On ModControllerFullyExecuted`))
          (bind _asbase_player_char (cast `/Game/Characters/BasePlayerChar` (`GameplayStatics.GetPlayerCharacter` 0) :!label _label_2))
          (`self.Client Continue Begin Play` _asbase_player_char)
          (`self.Server Continue Begin Play` _asbase_player_char))))))

(event `On ModControllerFullyExecuted`
  ;[0 1 0] Create ModControllerFullyExecuted Event
  (remove `/Game/Mods/TERPO-Reborn/MC_BP_TERPO.OnModControllerFullyExecuted` (`KismetArrayLibrary.Array_Get` (stale `self.ReceiveBeginPlay` _outactors)) (delegate `On ModControllerFullyExecuted`))
  (goto _label_2))

(event `Server Continue Begin Play`
  (params (BPC :type "/Game/Characters/BasePlayerChar Object Reference"))
  ;[1 0 0] Server
  (set `self.BPC` BPC)
  (bind _outactors (`GameplayStatics.GetAllActorsOfClass` "/Game/Mods/TERPO-Reborn/MC_BP_TERPO.MC_BP_TERPO_C"))
  (bind _item (`KismetArrayLibrary.Array_Get` _outactors))
  (`/Engine/EditorBlueprintResources/StandardMacros.IsValid` _item
    (:`Is Valid`
      (set `self.ModController` _item))))

(event `Client Continue Begin Play`
  (params (BPC :type "/Game/Characters/BasePlayerChar Object Reference"))
  ;[0 1 0] Client
  (set `self.BPC` BPC))

(fn `OnRep_Server Event is Called`)

(fn `SaveToDB`
  (params (playerId :type String) (oldSlot :type String) (newSlot :type String))
  (`KismetSystemLibrary.PrintString` playerId true true (struct :`G` 0.66 :`B` 1.0 :`A` 1.0) 10.0)
  (set `self.passToDB` (make `/Game/Mods/TERPO-Reborn/Variables/PassToDB_STRUCT_TERPO` playerId oldSlot newSlot))
  (`PersistenceComponent.SetDirty` (`/Game/Characters/BasePlayerChar.ConanCharacterPersistence` (`self.BPC`)) true 0.0))