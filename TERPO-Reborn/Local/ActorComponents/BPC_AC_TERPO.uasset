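; Player-character component for the TERPO mod that registers the character's name to its active slot and caches the player's slot names.
; On non-server BeginPlay, timers wait for the player character, setting component tick from KeepUIInVanityCam, and poll the controller's FCPC_AC_TERPO component for a valid player ID and slot.
; It then passes these with the character name to the MC_BP_TERPO mod controller and reads back the slot names.
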(event `Get Char Names`
  (params (PlayerId :type String) (ActiveSlot :type Integer) (CharacterName :type String))
  ;[1 0 0] Server execution path
  (bind _modcontrollerref (`self.GetValidModcontroller`)
    (:`Is Valid`
      (`/Game/Mods/TERPO-Reborn/Blueprints/MC_BP_TERPO.SetSlotName` _modcontrollerref PlayerId ActiveSlot CharacterName)
      (bind _slotnames (`/Game/Mods/TERPO-Reborn/Blueprints/MC_BP_TERPO.GetSlotNames` _modcontrollerref PlayerId))
      (set `self.CharacterNames` _slotnames))))

(event `self.ReceiveBeginPlay`
  ;[1 1 1] Client and Server execution path
  (if (`KismetSystemLibrary.IsServer`)
    ;[1 0 0] Server execution path
    (if (`KismetSystemLibrary.IsDedicatedServer`)
      _)
    (else
      ;[0 1 0] Client execution path
      (`self.SetComponentTickEnabled` true)
      (bind _returnvalue (`KismetSystemLibrary.K2_SetTimerDelegate` (delegate `WaitForValidPlayerController`) 0.5 true))
      (set `self.Timer` _returnvalue))))

(event `WaitForValidPlayerController`
  ;[0 1 0] Client execution path
  (`/Engine/EditorBlueprintResources/StandardMacros.IsValid` (`GameplayStatics.GetPlayerCharacter` 0)
    (:`Is Valid`
      (`KismetSystemLibrary.K2_ClearAndInvalidateTimerHandle` (`self.Timer`))
      (`self.SetComponentTickEnabled` (`self.KeepUI_InVanityCam`))
      (bind _asbase_player_char (`self.GetValidBPC`)
        (:`Is Valid BPC`
          (bind _returnvalue (`KismetSystemLibrary.K2_SetTimerDelegate` (delegate `Get FCPC_AC`) 1.0 true))
          (set `self.Timer` _returnvalue))))))

(event `Get FCPC_AC`
  ;[0 1 0] Client execution path
  (bind _fcpc_ac (`self.GetValidFCPC_AC`)
    (:`Is Valid`
      (bind _activesot (`/Game/Mods/TERPO-Reborn/ActorComponents/FCPC_AC_TERPO.GetActiveSlot` _fcpc_ac))
      (bind _playerid (`/Game/Mods/TERPO-Reborn/ActorComponents/FCPC_AC_TERPO.GetPlayerId` _fcpc_ac))
      (bind _charactername (`/Game/Characters/BaseBPChar.CharacterName` (stale `WaitForValidPlayerController` _asbase_player_char)))
      (if (and (>= (`KismetStringLibrary.Len` _playerid) 17) (> (`KismetStringLibrary.Len` _charactername) 0) (> _activesot 0) (<= _activesot 9))
        (`KismetSystemLibrary.K2_ClearAndInvalidateTimerHandle` (`self.Timer`))
        (`self.Get Char Names` _playerid _activesot _charactername)))))

(fn `GetHideUI`
  (returns (KeepUI_InVanityCam :type Boolean))
  (return (`self.KeepUI_InVanityCam`)))