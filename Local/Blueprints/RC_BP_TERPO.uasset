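; RCON command handler for the TERPO mod that lets server admins query and edit character slots and the time of day.
; RconCommand dispatches on the subcommand to handlers, which validate argument count and format before calling MCBPTERPORef, falling back to help text.
; Validation macros check numeric, Funcom ID and HH:MM:SS inputs, writing errors to the shared OutputStr reply.
; Slot listings are paged by array element, or by fixed-size chunks for JSON.
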(fn `getPageNumOrContents`
  (params (inputArr :type "Array of String") (Args :type "Array of String (by ref)"))
  (returns (returnStr :type String))
  (locals (out :type String) (input :type "Array of String"))
  (bind _returnvalue (`KismetArrayLibrary.Array_Length` inputArr))
  (bind _item (`KismetArrayLibrary.Array_Get` Args 2))
  (bind _returnvalue_2 (`KismetStringLibrary.Conv_StringToInt` _item))
  (set `local.input` inputArr)
  (if (> _returnvalue 1)
    (if (> (`KismetArrayLibrary.Array_Length` Args) 2)
      (if (`KismetStringLibrary.IsNumeric` _item)
        (`/Game/Systems/BP_MacroGlobal.And+Branch` (> _returnvalue_2 0) (<= _returnvalue_2 _returnvalue)
          (:`True`
            (bind _output_get (set `local.out` (`KismetArrayLibrary.Array_Get` (`local.input`) (- _returnvalue_2 1)))))
          (:`False`
            ;[1 1 1] Return number of pages
            (set `local.out` (`KismetStringLibrary.Concat_StrStr` "Pages: " (`KismetStringLibrary.Conv_IntToString` _returnvalue) "\nEnter TERPO getSlots <page num> to display that page") :!label _label)))
        (else
          (goto _label)))
      (else
        (goto _label)))
    (else
      ;[1 1 1] Return the first (and only) array element
      (set `local.out` (`KismetArrayLibrary.Array_Get` (`local.input`)))))
  (return _output_get))

(fn `getPageNumOrContentsJSON`
  (params (inputStr :type String) (Args :type "Array of String (by ref)"))
  (returns (returnStr :type String))
  (locals (out :type String))
  (bind _item (`KismetArrayLibrary.Array_Get` Args 2))
  (bind _returnvalue (`KismetStringLibrary.Len` inputStr))
  (set `local.out` inputStr)
  (if (> _returnvalue 4000)
    (if (> (`KismetArrayLibrary.Array_Length` Args) 2)
      (if (`KismetStringLibrary.IsNumeric` _item)
        (bind _output_get (set `local.out` (`KismetStringLibrary.GetSubstring` (`local.out`) (* (`KismetStringLibrary.Conv_StringToInt` _item) 4000) 4000)))
        (else
          ;[1 1 1] Return number of pages (as JSON string)
          (set `local.out` (`KismetStringLibrary.Concat_StrStr` "{\"chunks\": " (`KismetStringLibrary.Conv_IntToString` (/ _returnvalue 4000)) "}") :!label _label)))
      (else
        (goto _label))))
  (return _output_get))

(fn `partitionOutput`
  (params (input :type String))
  (returns (output :type "Array of String"))
  (locals (length :type Integer) (chunks :type Integer) (outputArr :type "Array of String") (inputStr :type String))
  (bind _output_get (set `local.inputStr` input))
  (set `local.length` (`KismetStringLibrary.Len` _output_get))
  (bind _output_get_2 (set `local.chunks` (/ (`local.length`) 4000)))
  (for _index (range (+ _output_get_2 1))
    (`KismetArrayLibrary.Array_Set` (`local.outputArr`) _index (`KismetStringLibrary.GetSubstring` (`local.inputStr`) (* _index 4000) 4000) true))
  ;[1 1 1] add header with number of chunks in case we have more than one
  (if (> (`local.chunks`) 0)
    (`KismetArrayLibrary.Array_Insert` (`local.outputArr`) (`KismetStringLibrary.Concat_StrStr` "{\"chunks\": " (`KismetStringLibrary.Conv_IntToString` (+ (`local.chunks`) 1)) "}")))
  ;[1 1 1] return the created array
  (return (`local.outputArr`)))

(fn `RconCommand`
  (params (world :type "World Object Reference") (args :type "Array of String (by ref)"))
  (returns (Output :type String) (ReturnValue :type Boolean))
  (locals (params :type "Array of String"))
  (bind _params (`local.params`))
  (bind _params_2 (`local.params`))
  (bind _params_3 (`local.params`))
  (bind _params_4 (`local.params`))
  (bind _params_5 (`local.params`))
  (bind _params_6 (`local.params`))
  (bind _params_7 (`local.params`))
  (bind _params_8 (`local.params`))
  (bind _item (`KismetArrayLibrary.Array_Get` _params 2))
  (bind _item_2 (`KismetArrayLibrary.Array_Get` _params_2 2))
  (bind _item_3 (`KismetArrayLibrary.Array_Get` _params_3 2))
  (bind _item_4 (`KismetArrayLibrary.Array_Get` _params_4 2))
  (bind _item_5 (`KismetArrayLibrary.Array_Get` _params_5 2))
  (bind _item_6 (`KismetArrayLibrary.Array_Get` _params_6 2))
  (bind _item_7 (`KismetArrayLibrary.Array_Get` _params_7 2))
  (bind _item_8 (`KismetArrayLibrary.Array_Get` _params_8 2))
  (bind _output_get (set `local.params` args))
  (`self.CommandReceived` _output_get)
  (switch `string` (`KismetArrayLibrary.Array_Get` _output_get 1)
    (:`Default`
      (set `self.outputStr` "usage:\n- TERPO getTime - returns current time on the server.\n- TERPO setTime [HH:MM:SS] - sets the time (24h format)\n- TERPO getSlots - returns the contents of the TERPO charSlots array.\n- TERPO getSlotsFuncomId || getSlotIdx - returns all slots registered for the given funcomId or index respectively.\n- TERPO delSlotsFuncomId || delSlotIdx - deletes all the information the mod has about the given funcomId or index respectively.\n- TERPO setSlotIdxName - set the Name of the character at the given slot.\n- TERPO setSlotIdxActive - set the character at the given slot to active and all other characters belonging to the same funcomId to inactive." :!label _label))
    (:`help`
      (goto _label))
    (:`getSlotsJSON`
      (bind _returnstr (`/Game/Mods/TERPO-Reborn/Blueprints/MC_BP_TERPO.getSlotsJSON` (`self.MC_BP_TERPO_Ref`)))
      (set `self.outputStr` (`self.getPageNumOrContentsJSON` _returnstr (`local.params`))))
    (:`getSlots`
      (bind _chunksout (`/Game/Mods/TERPO-Reborn/Blueprints/MC_BP_TERPO.getSlots` (`self.MC_BP_TERPO_Ref`)))
      (set `self.outputStr` (`self.getPageNumOrContents` _chunksout (`local.params`))))
    (:`getSlotIdx`
      (`self.checkHasNumArguments` 2 _params_4
        (:`true`
          (`self.checkIsNumeric` _item_4
            (:`true`
              (bind _output (`/Game/Mods/TERPO-Reborn/Blueprints/MC_BP_TERPO.getSlotIdx` (`self.MC_BP_TERPO_Ref`) (`KismetStringLibrary.Conv_StringToInt` _item_4)))
              (set `self.outputStr` _output))
            (:`false`
              _)))
        (:`false`
          _)))
    (:`getSlotsFuncomId`
      (`self.checkHasNumArguments` 2 _params_3
        (:`true`
          (`self.checkIsFuncomId` _item_3
            (:`true`
              (bind _output_2 (`/Game/Mods/TERPO-Reborn/Blueprints/MC_BP_TERPO.getSlotsFuncomId` (`self.MC_BP_TERPO_Ref`) _item_3))
              (set `self.outputStr` _output_2))
            (:`false`
              _)))
        (:`false`
          _)))
    (:`delSlotIdx`
      (`self.checkHasNumArguments` 2 _params_7
        (:`true`
          (`self.checkIsNumeric` _item_7
            (:`true`
              (bind _output_3 (`/Game/Mods/TERPO-Reborn/Blueprints/MC_BP_TERPO.delSlotIdx` (`self.MC_BP_TERPO_Ref`) (`KismetStringLibrary.Conv_StringToInt` _item_7)))
              (set `self.outputStr` _output_3))
            (:`false`
              _)))
        (:`false`
          _)))
    (:`delSlotsFuncomId`
      (`self.checkHasNumArguments` 2 _params
        (:`true`
          (`self.checkIsFuncomId` _item
            (:`true`
              (bind _output_4 (`/Game/Mods/TERPO-Reborn/Blueprints/MC_BP_TERPO.delSlotsFuncomId` (`self.MC_BP_TERPO_Ref`) _item))
              (set `self.outputStr` _output_4))
            (:`false`
              _)))
        (:`false`
          _)))
    (:`setSlotIdxName`
      (`self.checkHasNumArguments` 3 _params_8
        (:`true`
          (`self.checkIsNumeric` _item_8
            (:`true`
              (bind _output_5 (`/Game/Mods/TERPO-Reborn/Blueprints/MC_BP_TERPO.setSlotIdxName` (`self.MC_BP_TERPO_Ref`) (`KismetStringLibrary.Conv_StringToInt` _item_8) (`KismetArrayLibrary.Array_Get` _params_8 3)))
              (set `self.outputStr` _output_5))
            (:`false`
              _)))
        (:`false`
          _)))
    (:`setSlotIdxActive`
      (`self.checkHasNumArguments` 2 _params_2
        (:`true`
          (`self.checkIsNumeric` _item_2
            (:`true`
              (bind _output_6 (`/Game/Mods/TERPO-Reborn/Blueprints/MC_BP_TERPO.setSlotIdxActive` (`self.MC_BP_TERPO_Ref`) (`KismetStringLibrary.Conv_StringToInt` _item_2)))
              (set `self.outputStr` _output_6))
            (:`false`
              _)))
        (:`false`
          _)))
    (:`getTimeDecimal`
      (set `self.outputStr` (`KismetStringLibrary.Conv_DoubleToString` (`/Game/Mods/TERPO-Reborn/Blueprints/MC_BP_TERPO.getTimeDecimal` (`self.MC_BP_TERPO_Ref`)))))
    (:`getTime`
      (set `self.outputStr` (`/Game/Mods/TERPO-Reborn/Blueprints/MC_BP_TERPO.getTime` (`self.MC_BP_TERPO_Ref`))))
    (:`setTimeDecimal`
      (`self.checkHasNumArguments` 2 _params_5
        (:`true`
          (`self.checkIsNumeric` _item_5
            (:`true`
              (bind _returnvalue (`/Game/Mods/TERPO-Reborn/Blueprints/MC_BP_TERPO.setTimeDecimal` (`self.MC_BP_TERPO_Ref`) _item_5))
              (set `self.outputStr` _returnvalue))
            (:`false`
              _)))
        (:`false`
          _)))
    (:`setTime`
      (`self.checkHasNumArguments` 2 _params_6
        (:`true`
          (`self.checkIsTimeOfDayFormat` _item_6
            (:`true`
              (bind _returnvalue_2 (`/Game/Mods/TERPO-Reborn/Blueprints/MC_BP_TERPO.setTime` (`self.MC_BP_TERPO_Ref`) _item_6))
              (set `self.outputStr` _returnvalue_2))
            (:`false`
              _)))
        (:`false`
          _))))
  (return (`self.outputStr`) true))