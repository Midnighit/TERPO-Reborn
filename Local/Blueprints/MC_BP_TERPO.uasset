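; TERPO mod controller for Conan Exiles that merges the mod's data tables and manages persistent multi-character slots per Funcom ID.
; Slot changes mark the persistence component dirty, while queued slot switches reach PassToDB through a timer-throttled queue with padded IDs.
; It constructs an RCON object and provides text-returning slot admin and time-of-day functions.
; Clients link the TERPO menu to the in-game menu; listen servers toggle a Funcom ID widget with Shift+X.
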(event `DatabaseQueueElementAdded`
  ;[1 0 0] Server execution path
  (`self.SetActorTickEnabled` true)
  (bind _returnvalue (`KismetSystemLibrary.K2_SetTimer` null "ProcessDatabaseQueue" 0.5 true))
  (set `self.ThrottleDatabaseAccess` _returnvalue))

(event `Key|Shift+X`
  (params (Key :type "Key Structure" :default "AnyKey"))
  ;[1 0.5 0.5] Non-dedicated Server execution path
  (:`Pressed`
    (if (`self.is_hidden`)
      (bind _returnvalue (`|CreateWidget` "/Game/Mods/TERPO-Reborn/Widgets/FuncomID_W_TERPO.FuncomID_W_TERPO_C"))
      (bind _output_get (set `self.Widget_Ref` _returnvalue))
      (set `self.is_hidden` false)
      (`UserWidget.AddToViewport` _output_get 9999)
      (else
        (set `self.is_hidden` true)
        (`Widget.RemoveFromParent` (`self.Widget_Ref`))))))

(event `CommandReceived`
  (params (Params :type "Array of String (by ref)"))
  ;[1 1 1] Client and Server execution path
)

(event `self.ReceiveBeginPlay`
  ;[1 1 1] Client and Server execution path
  (bind _returnvalue (`|GenericCreateObject` "/Game/Mods/TERPO-Reborn/Blueprints/RC_BP_TERPO.RC_BP_TERPO_C" self self))
  (add `/Game/Mods/TERPO-Reborn/Blueprints/RC_BP_TERPO.CommandReceived` _returnvalue (delegate `CommandReceived`))
  (if (`KismetSystemLibrary.IsServer`)
    ;[1 0 0] Server execution path
    (if (not (`KismetSystemLibrary.IsDedicatedServer`))
      ;[1 0.5 0.5] Non-dedicated Server execution path
      (`self.EnableInput` (`GameplayStatics.GetPlayerController` 0)))
    (else
      ;[0 1 0] Client execution path
      (`self.SetActorTickEnabled` true)
      (bind _returnvalue_2 (`KismetSystemLibrary.K2_SetTimerDelegate` (delegate `WaitForValidPlayerController`) 0.5 true))
      (set `self.Timer` _returnvalue_2))))

(event `WaitForValidPlayerController`
  ;[0 1 0] Client execution path
  (`/Engine/EditorBlueprintResources/StandardMacros.IsValid` (`GameplayStatics.GetPlayerCharacter` 0)
    (:`Is Valid`
      (`KismetSystemLibrary.K2_ClearAndInvalidateTimerHandle` (`self.Timer`))
      (`self.SetActorTickEnabled` false)
      (bind _returnvalue (`GUIModuleController.GetModule` (`GUIModuleController.GetGUIModuleController`) "IngameMenu"))
      (add `GUIModule.SignalActivated` _returnvalue (delegate `IngameMenuOpened`)))))

(event `IngameMenuOpened`
  (params (module :type "GUIModule Object Reference") (isActive :type Boolean))
  ;[0 1 0] Client execution path
  (bind _returnvalue (`GUIModuleController.ActivateModule` (`GUIModuleController.GetGUIModuleController`) "MainMenu_TERPO" isActive false))
  (cast `/Game/Mods/TERPO-Reborn/Widgets/MainMenu_W_TERPO` _returnvalue))

(fn `AddLeadingZero`
  (params (String :type String))
  (returns (Output_Get :type String))
  (locals (outStr :type String))
  (if (== (`KismetStringLibrary.Len` String) 1)
    (set `local.outStr` (`KismetStringLibrary.Concat_StrStr` "0" String))
    (else
      (set `local.outStr` String)))
  (return (`local.outStr`)))

(fn `AddToDatabaseQueue`
  (params (queueElement :type "/Game/Mods/TERPO-Reborn/Variables/PassToDB_STRUCT_TERPO Structure"))
  (locals (idx :type Integer :default 0) (funcomId :type String))
  (bind (_funcomid _oldslot _newslot) (break `/Game/Mods/TERPO-Reborn/Variables/PassToDB_STRUCT_TERPO` queueElement))
  (bind _output_get (set `local.funcomId` _funcomid))
  (bind _output_get_2 (set `local.idx` (- 17 (`KismetStringLibrary.Len` _output_get))))
  (for _ (range 1 (+ _output_get_2 1))
    (set `local.funcomId` (`KismetStringLibrary.Concat_StrStr` (`local.funcomId`) "#")))
  (`KismetArrayLibrary.Array_Add` (`self.DatabaseQueue`) (make `/Game/Mods/TERPO-Reborn/Variables/PassToDB_STRUCT_TERPO` (`local.funcomId`) _oldslot _newslot))
  (`self.DatabaseQueueElementAdded`)
  (return))

(fn `convertHMS_toDecimal`
  (params (timeHMS :type String))
  (returns (ReturnValue :type "Float (double-precision)"))
  (bind (_lefts _rights) (`KismetStringLibrary.Split` timeHMS ":"))
  (bind (_lefts_2 _rights_2) (`KismetStringLibrary.Split` _rights ":"))
  (return (+ (`KismetStringLibrary.Conv_StringToDouble` _lefts) (/ (`KismetStringLibrary.Conv_StringToDouble` _lefts_2) 60.0) (/ (`KismetStringLibrary.Conv_StringToDouble` _rights_2) 3600.0))))

(fn `delSlotIdx`
  (params (Idx :type Integer))
  (returns (Output :type String))
  (locals (outputStr :type String))
  (if (> (`KismetArrayLibrary.Array_Length` (`self.charSlots`)) Idx)
    (`KismetArrayLibrary.Array_Remove` (`self.charSlots`) Idx)
    (bind _output_get (set `local.outputStr` (`KismetStringLibrary.Concat_StrStr` "Slot at Index " (`KismetStringLibrary.Conv_IntToString` Idx) " has been deleted.")))
    (else
      (set `local.outputStr` "Index out of bounds")))
  (return _output_get))

(fn `delSlotsFuncomId`
  (params (funcomId :type String))
  (returns (Output :type String))
  (locals (RemoveIdxList :type "Array of /Game/Mods/TERPO-Reborn/Variables/CharSlots_STRUCT_TERPO Structure"))
  ;[1 1 1] Determine which indexes need to be removed
  (for _array_element (`self.charSlots`)
    (if (`KismetStringLibrary.EqualEqual_StrStr` (`.funcomId_14_384CF29947A0DDCEDBFD55AFE1600E76` (break `/Game/Mods/TERPO-Reborn/Variables/CharSlots_STRUCT_TERPO` _array_element)) funcomId)
      (`KismetArrayLibrary.Array_Add` (`local.RemoveIdxList`) _array_element)))
  ;[1 1 1] Perform the actual removal of the elements
  (for _array_element_2 (`local.RemoveIdxList`)
    (`KismetArrayLibrary.Array_RemoveItem` (`self.charSlots`) _array_element_2))
  (return (`KismetStringLibrary.Concat_StrStr` "All slots for funcomId " funcomId " have been deleted.")))

(fn `GetActiveSlot`
  (params (funcomId :type String))
  (returns (index :type Integer) (slot :type Integer))
  (locals (arrayIndex :type Integer) (funcomIdFound :type Boolean))
  (bind _arrayindex (`local.arrayIndex`))
  (set `local.funcomIdFound` false) ; Initialize funcomIdFound\nto false
  (set `local.arrayIndex` -1) ; Initialze array\nindex to -1
  (for (_array_element _array_index) (`self.charSlots`)
    (bind (_funcomid _slotnum _slotname _isactive) (break `/Game/Mods/TERPO-Reborn/Variables/CharSlots_STRUCT_TERPO` _array_element))
    (if (`KismetStringLibrary.EqualEqual_StrStr` funcomId _funcomid)
      (if _isactive
        (set `local.arrayIndex` _array_index) ; Remember array\nindex of active slot
        (break)
        (else
          (set `local.funcomIdFound` true) ; Remember if funcomId was\nfound but not active slot
        ))))
  (if (>= _arrayindex 0)
    (return _arrayindex _slotnum) ; Array index was found
    (elif (not (`local.funcomIdFound`))
      (bind _returnvalue (`KismetArrayLibrary.Array_Add` (`self.charSlots`) (make `/Game/Mods/TERPO-Reborn/Variables/CharSlots_STRUCT_TERPO` funcomId 1 "" true))) ; Array index wasn't found.\n-> add new array element
      (`PersistenceComponent.SetDirty` (`self.PersistenceComponent`) true 5.0)
      (return _returnvalue 1)
      (else
        (`KismetSystemLibrary.PrintString` "TERPO: funcomId but no active slot found!" true true (struct :`R` 1.0 :`B` 0.016 :`A` 1.0) 30.0) ; funcomId found, active slot not found.\nShould never get here!!!
        (return -1 -1)))))

(fn `GetCharSlotConfig`
  (returns (Output :type "/Game/Mods/TERPO-Reborn/Variables/Settings/CharSlots_S_STRUCT_TERPO Structure"))
  (return (make `/Game/Mods/TERPO-Reborn/Variables/Settings/CharSlots_S_STRUCT_TERPO` (`self.ConfigMaxSlots`) (`self.ConfigMaxAdminSlots`))))

(fn `getSlotIdx`
  (params (Idx :type Integer))
  (returns (Output :type String))
  (locals (outputStr :type String))
  (bind (_funcomid _slotnum _slotname _isactive) (break `/Game/Mods/TERPO-Reborn/Variables/CharSlots_STRUCT_TERPO` (`KismetArrayLibrary.Array_Get` (`self.charSlots`) Idx)))
  (if (> (`KismetArrayLibrary.Array_Length` (`self.charSlots`)) Idx)
    (bind _output_get (set `local.outputStr` "Idx  | funcomId         | Slot | isActive | Name\n"))
    (bind _output_get_2 (set `local.outputStr` (`KismetStringLibrary.Concat_StrStr` _output_get (`KismetStringLibrary.LeftPad` (`KismetStringLibrary.Conv_IntToString` Idx) 4) " | " (`KismetStringLibrary.RightPad` _funcomid 16) " | " (`KismetStringLibrary.Conv_IntToString` _slotnum) "    | " (`KismetStringLibrary.RightPad` (`KismetStringLibrary.Conv_BoolToString` _isactive) 8) " | " _slotname)))
    (else
      (set `local.outputStr` "Index out of bounds")))
  (return _output_get_2))

(fn `GetSlotNames`
  (params (funcomId :type String))
  (returns (slotNames :type "Array of String"))
  (locals (CharNames :type "Array of String"))
  (for _array_element (`self.charSlots`)
    (bind ((`funcomId_14_384CF29947A0DDCEDBFD55AFE1600E76` _funcomid) (`slotNum_7_7D6E774649A86AD2234A9BA64B92E55B` _slotnum) (`slotName_11_ABDA33584EC80E7CE9033587B1F746D7` _slotname)) (break `/Game/Mods/TERPO-Reborn/Variables/CharSlots_STRUCT_TERPO` _array_element))
    (if (`KismetStringLibrary.EqualEqual_StrStr` funcomId _funcomid)
      (`KismetArrayLibrary.Array_Set` (`local.CharNames`) _slotnum _slotname true)))
  (return (`local.CharNames`)))

(fn `getSlots`
  (returns (chunksOut :type "Array of String"))
  (locals (charSlotsTable :type String) (chunks :type "Array of String"))
  (bind _chunks (`local.chunks`))
  (set `local.charSlotsTable` "Idx  | funcomId         | Slot | isActive | Name\n")
  (for (_array_element _array_index) (`self.charSlots`)
    (bind (_funcomid _slotnum _slotname _isactive) (break `/Game/Mods/TERPO-Reborn/Variables/CharSlots_STRUCT_TERPO` _array_element))
    (bind _returnvalue (`KismetStringLibrary.Concat_StrStr` (`KismetStringLibrary.LeftPad` (`KismetStringLibrary.Conv_IntToString` _array_index) 4) " | " (`KismetStringLibrary.RightPad` _funcomid 16) " | " (`KismetStringLibrary.Conv_IntToString` _slotnum) "    | " (`KismetStringLibrary.RightPad` (`KismetStringLibrary.Conv_BoolToString` _isactive) 8) " | " _slotname "\n"))
    ;[1 1 1] Assemble the full output array
    (if (<= (+ (`KismetStringLibrary.Len` _returnvalue) (`KismetStringLibrary.Len` (`local.charSlotsTable`))) 4000)
      (set `local.charSlotsTable` (`KismetStringLibrary.Concat_StrStr` (`local.charSlotsTable`) _returnvalue))
      (else
        (`KismetArrayLibrary.Array_Add` (`local.chunks`) (`local.charSlotsTable`))
        (set `local.charSlotsTable` _returnvalue))))
  (`KismetArrayLibrary.Array_Add` _chunks (`local.charSlotsTable`))
  (return _chunks))

(fn `getSlotsFuncomId`
  (params (funcomId :type String))
  (returns (Output :type String))
  (locals (charSlotsTable :type String))
  (set `local.charSlotsTable` "Idx  | funcomId         | Slot | isActive | Name\n")
  (for (_array_element _array_index) (`self.charSlots`)
    (bind (_funcomid _slotnum _slotname _isactive) (break `/Game/Mods/TERPO-Reborn/Variables/CharSlots_STRUCT_TERPO` _array_element))
    (if (`KismetStringLibrary.EqualEqual_StrStr` _funcomid funcomId)
      (set `local.charSlotsTable` (`KismetStringLibrary.Concat_StrStr` (`local.charSlotsTable`) (`KismetStringLibrary.LeftPad` (`KismetStringLibrary.Conv_IntToString` _array_index) 4) " | " (`KismetStringLibrary.RightPad` _funcomid 16) " | " (`KismetStringLibrary.Conv_IntToString` _slotnum) "    | " (`KismetStringLibrary.RightPad` (`KismetStringLibrary.Conv_BoolToString` _isactive) 8) " | " _slotname "\n"))))
  (return (`local.charSlotsTable`)))

(fn `getSlotsJSON`
  (returns (returnStr :type String))
  (locals (charSlotsJSON :type String))
  ;[1 1 1] Assemle the output JSON string
  (set `local.charSlotsJSON` "{\"slots\":[")
  (for _array_element (`self.charSlots`)
    (bind (_funcomid _slotnum _slotname _isactive) (break `/Game/Mods/TERPO-Reborn/Variables/CharSlots_STRUCT_TERPO` _array_element))
    (set `local.charSlotsJSON` (`KismetStringLibrary.Concat_StrStr` (`local.charSlotsJSON`) "{\"funcomId\":\"" _funcomid "\",\"slotNum\":" (`KismetStringLibrary.Conv_IntToString` _slotnum) ",\"slotName\":\"" _slotname "\",\"isActive\":" (`KismetStringLibrary.Conv_BoolToString` _isactive) "},")))
  (return (`KismetStringLibrary.Concat_StrStr` (`KismetStringLibrary.LeftChop` (`local.charSlotsJSON`) 1) "]}")))

(fn `getTime`
  (returns (ReturnValue :type String))
  (bind _returnvalue (`ConanTimeOfDayManager.GetTimeOfDay` (`self.GetTimeOfDayManagerRef`)))
  (bind _returnvalue_2 (`KismetMathLibrary.Round` (* 3600 (mod _returnvalue 1.0))))
  (return (`KismetStringLibrary.Concat_StrStr` (`KismetStringLibrary.Conv_IntToString` (`KismetMathLibrary.FFloor` _returnvalue)) ":" (`self.AddLeadingZero` (`KismetStringLibrary.Conv_IntToString` (/ _returnvalue_2 60))) ":" (`self.AddLeadingZero` (`KismetStringLibrary.Conv_IntToString` (mod _returnvalue_2 60))))))

(fn `getTimeDecimal`
  (returns (return :type "Float (double-precision)"))
  (locals (LocalTimer :type "TimerHandle Structure"))
  (bind _returnvalue (`ConanTimeOfDayManager.GetTimeOfDay` (`self.GetTimeOfDayManagerRef`)))
  (return _returnvalue))

(fn `GetTimeOfDayManagerRef`
  (returns (Item :type "ConanTimeOfDayManager Object Reference"))
  (bind _outactors (`GameplayStatics.GetAllActorsOfClass` "/Script/ConanSandbox.ConanTimeOfDayManager"))
  (bind _item (`KismetArrayLibrary.Array_Get` _outactors))
  (`/Engine/EditorBlueprintResources/StandardMacros.IsValid` _item
    (:`Is Valid`
      _)
    (:`Is Not Valid`
      (`LoggerLibrary.DWLogString` "TERPO (MC_BP): No valid TimeOfDayManager found." "GlobalServerChannel" "INFOL_IMPORTANT" true)))
  (return _item))

(fn `ModDataTableOperations`
  (`self.MergeDataTables` "/Game/UI/UIModuleTable.UIModuleTable" "/Game/Mods/TERPO-Reborn/Tables/UIModule_DT_TERPO.UIModule_DT_TERPO")
  (`self.MergeDataTables` "/Game/Items/Feats/FeatTable.FeatTable" "/Game/Mods/TERPO-Reborn/Tables/FeatTable_DT_TERPO.FeatTable_DT_TERPO")
  (`self.MergeDataTables` "/Game/Items/ItemTable.ItemTable" "/Game/Mods/TERPO-Reborn/Tables/ItemTable_DT_TERPO.ItemTable_DT_TERPO")
  (`self.MergeDataTables` "/Game/Items/Recipes/RecipesTable.RecipesTable" "/Game/Mods/TERPO-Reborn/Tables/RecipesTable_DT_TERPO.RecipesTable_DT_TERPO")
  (`self.MergeDataTables` "/Game/Sorcery/Spells/SpellTable.SpellTable" "/Game/Mods/TERPO-Reborn/Tables/SpellTable_DT_TERPO.SpellTable_DT_TERPO")
  (`self.MergeDataTables` "/Game/Items/ItemStatModificationTable.ItemStatModificationTable" "/Game/Mods/TERPO-Reborn/Tables/ItemStatModification_DT_TERPO.ItemStatModification_DT_TERPO"))

(fn `ProcessDatabaseQueue`
  (bind _databasequeue (`self.DatabaseQueue`))
  (set `self.passToDB` (`KismetArrayLibrary.Array_Get` (`self.DatabaseQueue`)))
  (`PersistenceComponent.SetDirty` (`self.PersistenceComponent`) true 0.1)
  (`KismetArrayLibrary.Array_Remove` _databasequeue)
  (if (== (`KismetArrayLibrary.Array_Length` _databasequeue) 0)
    (`KismetSystemLibrary.K2_ClearAndInvalidateTimerHandle` (`self.ThrottleDatabaseAccess`))
    (`self.SetActorTickEnabled` false)))

(fn `SetCharSlotsConfig`
  (params (Input :type "/Game/Mods/TERPO-Reborn/Variables/Settings/CharSlots_S_STRUCT_TERPO Structure"))
  (bind _output_get (set `self.ConfigMaxSlots` Input_CharSlots_4_E770209F414103B459EACBAE24026CEA))
  (if (<= (+ _output_get Input_AdminCharSlots_6_09E5E7594701ED202DB1F28C8D41E207) 9)
    (set `self.ConfigMaxAdminSlots` Input_AdminCharSlots_6_09E5E7594701ED202DB1F28C8D41E207)
    (else
      (set `self.ConfigMaxAdminSlots` (- 9 Input_CharSlots_4_E770209F414103B459EACBAE24026CEA))))
  (`PersistenceComponent.SetDirty` (`self.PersistenceComponent`) true 5.0))

(fn `SetSlotActive`
  (params (funcomId :type String) (slotNum :type Integer))
  (returns (index :type Integer))
  (locals (ArrayIndex :type Integer))
  (bind _charslots (`self.charSlots`))
  (set `local.ArrayIndex` -1) ; Initialze array\nindex to -1
  (for (_array_element _array_index) (`self.charSlots`)
    (bind ((`funcomId_14_384CF29947A0DDCEDBFD55AFE1600E76` _funcomid) (`slotNum_7_7D6E774649A86AD2234A9BA64B92E55B` _slotnum) (`slotName_11_ABDA33584EC80E7CE9033587B1F746D7` _slotname)) (break `/Game/Mods/TERPO-Reborn/Variables/CharSlots_STRUCT_TERPO` _array_element))
    (if (`KismetStringLibrary.EqualEqual_StrStr` funcomId _funcomid)
      (if (== slotNum _slotnum)
        (`KismetArrayLibrary.Array_Set` _charslots _array_index (make `/Game/Mods/TERPO-Reborn/Variables/CharSlots_STRUCT_TERPO` _funcomid _slotnum _slotname true)) ; Correct slot, set to active
        (set `local.ArrayIndex` _array_index) ; Remember array index
        (else
          (`KismetArrayLibrary.Array_Set` _charslots _array_index (make `/Game/Mods/TERPO-Reborn/Variables/CharSlots_STRUCT_TERPO` _funcomid _slotnum _slotname false)) ; Wrong slot, set to inactive
        ))))
  (if (>= (`local.ArrayIndex`) 0)
    (`PersistenceComponent.SetDirty` (`self.PersistenceComponent`) true 0.5)
    (return (`local.ArrayIndex`)) ; Array index was found
    (else
      (bind _returnvalue (`KismetArrayLibrary.Array_Add` (`self.charSlots`) (make `/Game/Mods/TERPO-Reborn/Variables/CharSlots_STRUCT_TERPO` funcomId slotNum "" true))) ; Array index wasn't found\n-> add new array element
      (`PersistenceComponent.SetDirty` (`self.PersistenceComponent`) true 0.5)
      (return _returnvalue))))

(fn `setSlotIdxActive`
  (params (Idx :type Integer))
  (returns (Output :type String))
  (locals (outputStr :type String) (funcom_id :type String) (ActiveIdx :type Integer) (ArrayIdx :type Integer))
  (bind _charslots (`self.charSlots`))
  (bind _arrayidx (`local.ArrayIdx`))
  (if (> (`KismetArrayLibrary.Array_Length` (`self.charSlots`)) Idx)
    (set `local.ActiveIdx` Idx)
    (set `local.funcom_id` (`.funcomId_14_384CF29947A0DDCEDBFD55AFE1600E76` (break `/Game/Mods/TERPO-Reborn/Variables/CharSlots_STRUCT_TERPO` (`KismetArrayLibrary.Array_Get` (`self.charSlots`) Idx))))
    ;[1 1 1] Set all slots belonging to given funcom_id except the one given to inactive
    (for (_array_element _array_index) (`self.charSlots`)
      (set `local.ArrayIdx` _array_index)
      (bind ((`funcomId_14_384CF29947A0DDCEDBFD55AFE1600E76` _funcomid) (`slotNum_7_7D6E774649A86AD2234A9BA64B92E55B` _slotnum) (`slotName_11_ABDA33584EC80E7CE9033587B1F746D7` _slotname)) (break `/Game/Mods/TERPO-Reborn/Variables/CharSlots_STRUCT_TERPO` _array_element))
      (if (`KismetStringLibrary.EqualEqual_StrStr` _funcomid (`local.funcom_id`))
        (if (== (`local.ArrayIdx`) (`local.ActiveIdx`))
          (`KismetArrayLibrary.Array_Set` _charslots _arrayidx (make `/Game/Mods/TERPO-Reborn/Variables/CharSlots_STRUCT_TERPO` _funcomid _slotnum _slotname true))
          (else
            (`KismetArrayLibrary.Array_Set` _charslots _arrayidx (make `/Game/Mods/TERPO-Reborn/Variables/CharSlots_STRUCT_TERPO` _funcomid _slotnum _slotname false))))))
    (bind _output_get (set `local.outputStr` (`KismetStringLibrary.Concat_StrStr` "Character at index " (`KismetStringLibrary.Conv_IntToString` Idx) " has been set to active slot.")))
    (else
      (set `local.outputStr` "Index out of bounds.")))
  (return _output_get))

(fn `setSlotIdxName`
  (params (Idx :type Integer) (Name :type String))
  (returns (Output :type String))
  (locals (outputStr :type String))
  (bind ((`funcomId_14_384CF29947A0DDCEDBFD55AFE1600E76` _funcomid) (`slotNum_7_7D6E774649A86AD2234A9BA64B92E55B` _slotnum) (`isActive_12_F24C2E1247D5EE22ACB7B79917AFBD77` _isactive)) (break `/Game/Mods/TERPO-Reborn/Variables/CharSlots_STRUCT_TERPO` (`KismetArrayLibrary.Array_Get` (`self.charSlots`) Idx)))
  (if (> (`KismetArrayLibrary.Array_Length` (`self.charSlots`)) Idx)
    (`KismetArrayLibrary.Array_Set` (`self.charSlots`) Idx (make `/Game/Mods/TERPO-Reborn/Variables/CharSlots_STRUCT_TERPO` _funcomid _slotnum Name _isactive))
    (bind _output_get (set `local.outputStr` (`KismetStringLibrary.Concat_StrStr` "Name of character at index " (`KismetStringLibrary.Conv_IntToString` Idx) " has been changed to " Name ".")))
    (else
      (set `local.outputStr` "Index out of bounds")))
  (return _output_get))

(fn `SetSlotName`
  (params (funcomId :type String) (slotNum :type Integer) (characterName :type String))
  (returns (index :type Integer))
  (locals (ArrayIndex :type Integer) (charSlotsStrDEBUG :type String))
  (set `local.ArrayIndex` -1) ; Initialze array\nindex to -1
  (for (_array_element _array_index) (`self.charSlots`)
    (bind (_funcomid _slotnum _slotname _isactive) (break `/Game/Mods/TERPO-Reborn/Variables/CharSlots_STRUCT_TERPO` _array_element))
    (`/Game/Systems/BP_MacroGlobal.And+Branch` (== slotNum _slotnum) (`KismetStringLibrary.EqualEqual_StrStr` funcomId _funcomid) ; funcomId and slot\nmatch those given.
      (:`True`
        (`KismetArrayLibrary.Array_Set` (`self.charSlots`) _array_index (make `/Game/Mods/TERPO-Reborn/Variables/CharSlots_STRUCT_TERPO` _funcomid _slotnum characterName _isactive) true)
        (set `local.ArrayIndex` _array_index) ; Remember array index
        (break))))
  (if (not (>= (`local.ArrayIndex`) 0))
    (bind _returnvalue (`KismetArrayLibrary.Array_Add` (`self.charSlots`) (make `/Game/Mods/TERPO-Reborn/Variables/CharSlots_STRUCT_TERPO` funcomId slotNum characterName true)))
    (set `local.ArrayIndex` _returnvalue))
  (`PersistenceComponent.SetDirty` (`self.PersistenceComponent`) true 0.5)
  (return (`local.ArrayIndex`)) ; Array index was found
)

(fn `setTime`
  (params (timeHMS :type String))
  (returns (ReturnValue :type String))
  (`ConanTimeOfDayManager.SetTimeOfDay` (`self.GetTimeOfDayManagerRef`) (`self.convertHMS_toDecimal` timeHMS))
  (return (`KismetStringLibrary.Concat_StrStr` "Time has been set to " timeHMS ".")))

(fn `setTimeDecimal`
  (params (NewTimeOfDay :type String))
  (returns (ReturnValue :type String))
  (`ConanTimeOfDayManager.SetTimeOfDay` (`self.GetTimeOfDayManagerRef`) (`KismetStringLibrary.Conv_StringToDouble` NewTimeOfDay))
  (return (`KismetStringLibrary.Concat_StrStr` "Time has been set to " NewTimeOfDay ".")))

(fn `UserConstructionScript`)